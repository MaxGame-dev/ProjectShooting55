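; AI controller that gives its controlled BP_MyCharacter a target when perception picks up a player-owned actor.
; BeginPlay casts and caches the controlled pawn.
; On each perception update, it identifies player actors by searching the owner's display name for "PlayerController" and passes them to SetTargetCharacter.
; It does not check whether the actor was sensed or lost, and never clears the target itself.
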(event OnPerceptionUpdated(AIPerception)
  (params (UpdatedActors :type Array%20of%20Actor%20Object%20References))
  (Utilities|IsValid (Variables|Default|GetMyCharacter)
    (:Is%20Valid
      (for _array_element UpdatedActors
        (if (Utilities|String|Contains (Utilities|GetDisplayName (Components|GetOwner _array_element)) "PlayerController")
          (Default|SetTargetCharacter (Variables|Default|GetMyCharacter) _array_element))))))

(event EventBeginPlay
  (bind _returnvalue (Pawn|GetControlledPawn))
  (bind _asbp_my_character (Utilities|Casting|CastToBP_MyCharacter _returnvalue))
  (Utilities|IsValid _asbp_my_character
    (:Is%20Valid
      (Variables|Default|SetMyCharacter _asbp_my_character))))

(fn ConstructionScript)