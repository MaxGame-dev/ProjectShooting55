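; Shared character for the player and AI enemies, with twin ammo counters, a weapon component and HP.
; BeginPlay branches on controller type: players get input and HUD, AI gets a looping timer that turns toward its target and auto-fires.
; The first dodge press starts constant forward movement; later presses do timer-driven dashes alongside strafing.
; Damage updates HP gauges; death, also triggered by ramming, hides meshes, explodes and may spawn BP_Bullet.
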(event OnComponentHit(CapsuleComponent)
  (params (HitComponent :type Primitive%20Component%20Object%20Reference) (OtherActor :type Actor%20Object%20Reference) (OtherComp :type Primitive%20Component%20Object%20Reference) (NormalImpulse :type Vector :default "0, 0, 0") (Hit :type Hit%20Result%20Structure%20%28by%20ref%29))
  (bind _returnvalue (Components|GetOwner OtherComp))
  (bind _returnvalue_2 (Utilities|GetDisplayName _returnvalue))
  ;[1 1 1] 敵にあたると爆発
  (if (and (Utilities|String|Contains _returnvalue_2 "MyCharacter") (Utilities|Enum|NotEqual(Enum) _returnvalue_2 (Utilities|GetDisplayName (Game|Player|GetPlayerPawn 0))))
    (Utilities|FlowControl|DoOnce false
      (:Completed
        (Game|Damage|ApplyDamage self 5e+02 0 0)))))

(event Custom|CheckDeadFalling
  ;[1 1 1] ダメージ受け処理
  (if (not (AI|Components|NavMovement|IsFalling (Variables|Character|GetCharacterMovement)))
    (Utilities|Time|ClearandInvalidateTimerbyHandle (stale Game|Damage|EventAnyDamage _returnvalue_2))
    (Collision|SetCollisionEnabled (Variables|Collision|GetCapsuleComponent) "NoCollision")))

(event Custom|StartMove
  ;[1 1 1] ゲームスタート、回避
  (Pawn|Input|AddMovementInput (Math|Vector|GetForwardVector (Math|Rotator|MakeRotator 0.0 0.0 (.yaw (Pawn|GetControlRotation :!class /Script/Engine.Pawn)))) 0.5 false))

(event Custom|UpdateDodgeAmount
  (bind _returnvalue (Transformation|GetActorLocation))
  (bind _returnvalue_2 (Transformation|GetActorRotation))
  (bind _dodgeamount (Variables|Movement|GetDodgeAmount))
  ;[1 1 1] ゲームスタート、回避
  (bind _output_get (Variables|Movement|SetDodgeTimer (+ (Variables|Movement|GetDodgeTimer) (Utilities|Time|GetWorldDeltaSeconds))))
  (if (>= _output_get 0.12)
    (Utilities|Time|ClearandInvalidateTimerbyHandle (stale Input|EnhancedActionEvents|EnhancedInputActionIA_MyDodge _returnvalue))
    (Utilities|FlowControl|DoOnce false) ; enters at Reset
    (else
      (Transformation|SetActorLocation (Math|Vector|Lerp(Vector) _returnvalue (+ _returnvalue (* (* (Math|Vector|GetForwardVector _returnvalue_2) _dodgeamount) (Variables|Movement|GetDodgeValueY)) (* (* (Math|Vector|GetRightVector _returnvalue_2) _dodgeamount) (Variables|Movement|GetDodgeValueX))) 0.05) true false))))

(event Custom|CheckTargetCharacter
  (bind _returnvalue (Transformation|GetActorRotation))
  (bind _returnvalue_2 (Transformation|GetActorLocation))
  (bind _weaponcomponent (Variables|Default|GetWeaponComponent))
  (bind _targetcharacter (Variables|AI|GetTargetCharacter))
  (bind _returnvalue_3 (Transformation|GetActorLocation _targetcharacter))
  (bind _returnvalue_4 (Math|Rotator|FindLookatRotation _returnvalue_2 _returnvalue_3))
  ;[1 1 1] ターゲットの方向を見て射撃するAI
  (Utilities|IsValid _targetcharacter
    (:Is%20Valid
      (if (Utilities|Operators|NotEqual(!=) _returnvalue _returnvalue_4 1.0)
        (Transformation|SetActorRotation (Math|Interpolation|RInterpTo _returnvalue _returnvalue_4 0.01 5.0))
        (elif (> (Variables|BP_MyCharacter_C|GetHp (Variables|AI|GetTargetCharacter)) 0.0)
          (if (Variables|AI|GetIsAutoShoot)
            (Utilities|FlowControl|DoOnce false :!label _label
              (:Completed
                (if (> (Variables|PlayerData|GetHp) 0.0)
                  (if (and (<= (Math|Random|RandomIntegerinRange 1 100) 50) (> (Variables|Weapon|GetWeaponType) 1))
                    (Default|EnemyLeftShoot _weaponcomponent)
                    (else
                      (Default|EnemyRightShoot _weaponcomponent)))
                  (Utilities|FlowControl|Delay 0.8)
                  (goto _label Reset)))))
          (else
            (CallFunction|EndCheckTargetCharacter)))))))

(event Custom|EndCheckTargetCharacter
  ;[1 1 1] 初期化処理
  (Utilities|Time|ClearandInvalidateTimerbyHandle (stale EventBeginPlay _returnvalue_3)))

(event Input|EnhancedActionEvents|EnhancedInputActionIA_MyMove
  (params (ActionValue :type Vector%202D%20Structure) (ElapsedSeconds :type Float%20%28double-precision%29) (TriggeredSeconds :type Float%20%28double-precision%29) (InputAction :type Input%20Action%20Object%20Reference :default "/Game/Project/Blueprints/Input/Actions/IA_MyMove.IA_MyMove"))
  (bind _returnvalue (Pawn|GetControlRotation :!class /Script/Engine.Pawn))
  ;[1 1 1] 移動入力
  (:Triggered
    (Variables|Movement|SetMoveValueX (.x ActionValue))
    (Pawn|Input|AddMovementInput (Math|Vector|GetRightVector (Math|Rotator|MakeRotator (.roll _returnvalue) 0.0 (.yaw _returnvalue))) (.x ActionValue) false))
  (:Completed
    (Variables|Movement|SetMoveValueX 0.0)
    (Variables|Movement|SetMoveValueY 0.0)))

(event Input|EnhancedActionEvents|EnhancedInputActionIA_MyDodge
  (params (ActionValue :type Boolean) (ElapsedSeconds :type Float%20%28double-precision%29) (TriggeredSeconds :type Float%20%28double-precision%29) (InputAction :type Input%20Action%20Object%20Reference :default "/Game/Project/Blueprints/Input/Actions/IA_MyDodge.IA_MyDodge"))
  ;[1 1 1] ゲームスタート、回避
  (:Started
    (if (Variables|Default|GetbMoveStart)
      (if (or (!= (Variables|Movement|GetMoveValueX) 0.0) (!= (Variables|Movement|GetMoveValueY) 0.0))
        (Utilities|FlowControl|DoOnce false
          (:Completed
            (Utilities|FlowControl|Sequence
              (:then_0
                (Audio|PlaySoundatLocation "/Game/FuturisticCombatAudioPack/Shut_Down_v1/Sounds/Shut_Down_v1_wav.Shut_Down_v1_Wav" (Transformation|GetActorLocation) "0, 0, 0" 1.0 1.5 0.0 0 0 0 0))
              (:then_1
                (Variables|Movement|SetDodgeValueX (Variables|Movement|GetMoveValueX))
                (Variables|Movement|SetDodgeValueY (Variables|Movement|GetMoveValueY))
                (Variables|Movement|SetDodgeTimer 0.0)
                (Utilities|FlowControl|Delay 0.2)
                (bind _returnvalue (Utilities|Time|SetTimerbyEvent (delegate Custom|UpdateDodgeAmount) (Utilities|Time|GetWorldDeltaSeconds) true)))))))
      (else
        (Variables|Default|SetbMoveStart true)
        (Utilities|Time|SetTimerbyEvent (delegate Custom|StartMove) (Utilities|Time|GetWorldDeltaSeconds) true)))))

(event Input|EnhancedActionEvents|EnhancedInputActionIA_MyReset
  (params (ActionValue :type Boolean) (ElapsedSeconds :type Float%20%28double-precision%29) (TriggeredSeconds :type Float%20%28double-precision%29) (InputAction :type Input%20Action%20Object%20Reference :default "/Game/Project/Blueprints/Input/Actions/IA_MyReset.IA_MyReset"))
  ;[1 1 1] とりあえずリセット
  (:Started
    (bind _returnvalue (Game|GetCurrentLevelName true))
    (Game|OpenLevel(byName) (Utilities|String|StringToName _returnvalue))))

(event Game|Damage|EventAnyDamage
  (params (Damage :type Float%20%28single-precision%29) (DamageType :type Damage%20Type%20Object%20Reference) (InstigatedBy :type Controller%20Object%20Reference) (DamageCauser :type Actor%20Object%20Reference))
  (bind _overheadgauge (Variables|Default|GetOverheadGauge))
  (bind _returnvalue (UserInterface|GetUserWidgetObject _overheadgauge))
  (bind _asoverhead_gauge (Utilities|Casting|CastToOverheadGauge _returnvalue))
  ;[1 1 1] ダメージ受け処理
  (Variables|PlayerData|SetHp (Math|Float|Max(Float) (- (Variables|PlayerData|GetHp) Damage) 0.0))
  (if (Variables|AI|GetIsAi)
    (Rendering|SetVisibility _overheadgauge true true)
    (Utilities|FlowControl|Sequence
      (:then_0
        (if (<= (Variables|PlayerData|GetHp) 0.0) :!label _label
          (CallFunction|EndCheckTargetCharacter)
          (Audio|PlaySoundatLocation "/Game/StarterContent/Audio/Explosion01.Explosion01" (Transformation|GetActorLocation) "0, 0, 0" 1.0 1.0 0.0 0 0 0 0)
          (Utilities|FlowControl|Sequence
            (:then_0
              (Rendering|SetVisibility (Variables|Default|GetRootMesh) false false))
            (:then_1
              (Collision|SetCollisionEnabled (Variables|Default|GetRootMesh) "NoCollision")
              (bind _returnvalue_2 (Utilities|Time|SetTimerbyEvent (delegate Custom|CheckDeadFalling) (Utilities|Time|GetWorldDeltaSeconds) true)))
            (:then_2
              (Components|Activation|SetActive (Variables|Default|GetParticleSystem) true true)
              (if (<= (Math|Random|RandomIntegerinRange 1 100) 50)
                (Game|SpawnActorfromClass "/Game/Project/Blueprints/MyCharacter/BP_Bullet.BP_Bullet_C" (Transformation|GetActorTransform) "Undefined" "MultiplyWithRoot" 0 0))))))
      (:then_1
        (Utilities|IsValid _asoverhead_gauge
          (:Is%20Valid
            (Default|SetOverheadhpGuage _asoverhead_gauge (Variables|PlayerData|GetHp) (Variables|PlayerData|GetMaxHp))
            (Utilities|FlowControl|Delay 2.0)
            (Rendering|SetVisibility (Variables|Default|GetOverheadGauge) false false)))))
    (else
      (CallFunction|UpdatePlayerHpUI)
      (goto _label))))

(event EventBeginPlay
  ;[1 1 1] 初期化処理
  (Variables|PlayerData|SetHp (Variables|PlayerData|GetMaxHp))
  (Variables|PlayerData|SetRemainingBullet1 (Variables|PlayerData|GetMaxBullet1))
  (Variables|PlayerData|SetRemainingBullet2 (Variables|PlayerData|GetMaxBullet2))
  (bind _asプレイヤーコントローラー (Utilities|Casting|CastToPlayerController (Pawn|GetController))
    (:then
      (Utilities|IsValid (PlayerController|LocalPlayerSubsystems|GetEnhancedInputLocalPlayerSubsystem _asプレイヤーコントローラー)
        (:Is%20Valid
          (Input|AddMappingContext (PlayerController|LocalPlayerSubsystems|GetEnhancedInputLocalPlayerSubsystem _asプレイヤーコントローラー) "/Game/Project/Blueprints/Input/IMC_MyDefault.IMC_MyDefault" 0 "(bIgnoreAllPressedKeysUntilRelease=True,bForceImmediately=False,bNotifyUserSettings=False)")
          (Utilities|FlowControl|Sequence
            (:then_0
              (bind _returnvalue (AddComponent|AddBPMyWeaponComponent false))
              (Variables|Default|SetWeaponComponent _returnvalue)
              (bind _returnvalue_2 (UserInterface|CreateWidget "/Game/Project/Blueprints/Widgets/PlayerGameUI.PlayerGameUI_C"))
              (Variables|UI|SetPlayerGameUI _returnvalue_2)
              (UserInterface|Viewport|AddtoViewport _returnvalue_2 0)
              (Default|SetRemainingBullet (Variables|UI|GetPlayerGameUI) 1 (Variables|PlayerData|GetRemainingBullet1))
              (Default|SetRemainingBullet (Variables|UI|GetPlayerGameUI) 2 (Variables|PlayerData|GetRemainingBullet2))
              (CallFunction|UpdatePlayerHpUI))
            (:then_1
              (CallFunction|ChangeCameraLock)
              (if (Variables|Camera|GetIsCameraLock)
                (Variables|Default|SetbUseControllerRotationYaw true)
                (Variables|/Script/Engine.CharacterMovementComponent|SetbOrientRotationToMovement (Variables|Character|GetCharacterMovement) false)
                (Variables|/Script/Engine.SpringArmComponent|SetbUsePawnControlRotation (Variables|Default|GetSpringArm) false)))))))
    (:CastFailed
      (bind _output_get (Variables|AI|SetIsAi true))
      (if _output_get
        (bind _returnvalue_3 (Utilities|Time|SetTimerbyFunctionName 0 "CheckTargetCharacter" 0.01 true))
        (bind _returnvalue_4 (AddComponent|AddBPMyWeaponComponent false))
        (Variables|Default|SetWeaponComponent _returnvalue_4)
        (bind _output_get_2 (Variables|PlayerData|SetMaxHp 1e+02))
        (Variables|PlayerData|SetHp _output_get_2)))))

(fn ConstructionScript)

(fn UpdatePlayerHpUI
  (bind _playergameui (Variables|UI|GetPlayerGameUI))
  (Utilities|IsValid _playergameui
    (:Is%20Valid
      (Default|SetHpGauge _playergameui (Variables|PlayerData|GetHp) (Variables|PlayerData|GetMaxHp)))))

(fn ChangeCameraLock
  (if (Variables|Camera|GetIsCameraLock)
    (Variables|Camera|SetIsCameraLock false)
    (else
      (Variables|Camera|SetIsCameraLock true))))

(fn SetTargetCharacter
  (params (TargetActor :type Actor%20Object%20Reference))
  (bind _asbp_my_character (Utilities|Casting|CastToBP_MyCharacter TargetActor))
  (Utilities|IsValid _asbp_my_character
    (:Is%20Valid
      (if (== (Variables|AI|GetTargetCharacter) 0)
        (Variables|AI|SetTargetCharacter _asbp_my_character)
        (else
          (Variables|AI|SetTargetCharacter 0))))))

(fn DecreaseRemainingBullet
  (params (WeaponType :type Integer))
  (bind _playergameui (Variables|UI|GetPlayerGameUI))
  (bind _playergameui_2 (Variables|UI|GetPlayerGameUI))
  (switch int WeaponType
    (:1
      (bind _output_get (Variables|PlayerData|SetRemainingBullet1 (- (Variables|PlayerData|GetRemainingBullet1) 1)))
      (Utilities|IsValid _playergameui_2
        (:Is%20Valid
          (Default|SetRemainingBullet _playergameui_2 1 _output_get))))
    (:2
      (bind _output_get_2 (Variables|PlayerData|SetRemainingBullet2 (- (Variables|PlayerData|GetRemainingBullet2) 1)))
      (Utilities|IsValid _playergameui
        (:Is%20Valid
          (Default|SetRemainingBullet _playergameui 2 _output_get_2))))))