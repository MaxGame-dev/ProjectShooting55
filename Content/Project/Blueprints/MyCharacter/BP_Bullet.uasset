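; BP_Bullet is an ammo pickup that refills both of the player's weapon types when touched.
; On sphere overlap, it matches the other actor to player pawn 0 by display name, then casts it to BP_MyCharacter.
; It adds a fixed amount to each remaining-bullet count, pushes both values to the player's game UI, then destroys itself.
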(event OnComponentBeginOverlap(Sphere)
  (params (OverlappedComponent :type Primitive%20Component%20Object%20Reference) (OtherActor :type Actor%20Object%20Reference) (OtherComp :type Primitive%20Component%20Object%20Reference) (OtherBodyIndex :type Integer) (bFromSweep :type Boolean) (SweepResult :type Hit%20Result%20Structure%20%28by%20ref%29))
  (if (Utilities|Enum|Equal(Enum) (Utilities|GetDisplayName OtherActor) (Utilities|GetDisplayName (Game|Player|GetPlayerPawn 0)))
    (bind _asbp_my_character (Utilities|Casting|CastToBP_MyCharacter OtherActor))
    (Utilities|FlowControl|Sequence
      (:then_0
        (bind _output_get (Variables|/Game/Project/Blueprints/MyCharacter/BP_MyCharacter.BP_MyCharacter_C|SetRemainingBullet1 _asbp_my_character (+ (Variables|/Game/Project/Blueprints/MyCharacter/BP_MyCharacter.BP_MyCharacter_C|GetRemainingBullet1 _asbp_my_character) 3)))
        (Default|SetRemainingBullet (Variables|/Game/Project/Blueprints/MyCharacter/BP_MyCharacter.BP_MyCharacter_C|GetPlayerGameUI _asbp_my_character) 1 _output_get))
      (:then_1
        (bind _output_get_2 (Variables|/Game/Project/Blueprints/MyCharacter/BP_MyCharacter.BP_MyCharacter_C|SetRemainingBullet2 _asbp_my_character (+ (Variables|/Game/Project/Blueprints/MyCharacter/BP_MyCharacter.BP_MyCharacter_C|GetRemainingBullet2 _asbp_my_character) 3)))
        (Default|SetRemainingBullet (Variables|/Game/Project/Blueprints/MyCharacter/BP_MyCharacter.BP_MyCharacter_C|GetPlayerGameUI _asbp_my_character) 2 _output_get_2))
      (:then_2
        (Actor|DestroyActor)))))

(fn ConstructionScript)