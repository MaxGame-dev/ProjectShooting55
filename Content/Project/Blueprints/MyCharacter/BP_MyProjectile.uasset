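; BP_MyProjectile is a projectile that resolves a single hit, pushing physics objects or damaging characters.
; A DoOnce-gated Hit event ignores the owner, applies a velocity-scaled impulse to simulating components, or applies damage when a "Damage"-tagged component's actor casts to BP_MyCharacter.
; DeleteProjectile hides the sphere, restarts the particle system and destroys the actor after a brief delay.
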(event Collision|EventHit
  (params (MyComp :type Primitive%20Component%20Object%20Reference) (Other :type Actor%20Object%20Reference) (OtherComp :type Primitive%20Component%20Object%20Reference) (bSelfMoved :type Boolean) (HitLocation :type Vector :default "0, 0, 0") (HitNormal :type Vector :default "0, 0, 0") (NormalImpulse :type Vector :default "0, 0, 0") (Hit :type Hit%20Result%20Structure%20%28by%20ref%29))
  (Utilities|FlowControl|DoOnce false
    (:Completed
      (if (!= Other (Components|GetOwner))
        (Variables|Default|SetHitActor Other)
        (bind _output_get (Variables|Default|SetHitComponent OtherComp))
        (Utilities|IsValid _output_get
          (:Is%20Valid
            (if (Physics|IsSimulatingPhysics _output_get "None")
              (Physics|AddImpulseatLocation (Variables|Default|GetHitComponent) (* (Transformation|GetVelocity) 1e+02) (Transformation|GetActorLocation) "None")
              (Utilities|DeleteProjectile)
              (else
                (Utilities|IsValid (Variables|Default|GetHitComponent)
                  (:Is%20Valid
                    (if (Components|ComponentHasTag (Variables|Default|GetHitComponent) "Projectile")
                      (Utilities|DeleteProjectile)
                      (elif (Components|ComponentHasTag (Variables|Default|GetHitComponent) "Damage")
                        (bind _asbp_my_character (Utilities|Casting|CastToBP_MyCharacter (Variables|Default|GetHitActor)))
                        (Game|Damage|ApplyDamage _asbp_my_character (Variables|Default|GetBaseDamage) 0 0)
                        (Utilities|DeleteProjectile)
                        (else
                          (Utilities|DeleteProjectile))))))))))))))

(fn ConstructionScript)