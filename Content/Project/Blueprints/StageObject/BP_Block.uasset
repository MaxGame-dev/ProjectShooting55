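; BP_Block is a stage block actor that explodes when hit by a projectile and can optionally move on its own.
; With IsAutoMove set, it disables mesh physics and, after a short delay, the AutoMove timeline offsets the mesh along relative X from its start location.
; Hits from actors with "Projectile" in their display name trigger particles and sound, hide the mesh, then destroy the actor after a delay.
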(event OnComponentHit(StaticMesh)
  (params (HitComponent :type Primitive%20Component%20Object%20Reference) (OtherActor :type Actor%20Object%20Reference) (OtherComp :type Primitive%20Component%20Object%20Reference) (NormalImpulse :type Vector :default "0, 0, 0") (Hit :type Hit%20Result%20Structure%20%28by%20ref%29))
  (if (Utilities|String|Contains (Utilities|GetDisplayName OtherActor) "Projectile")
    (Components|Activation|SetActive (Variables|Default|GetParticleSystem) true true)
    (Rendering|SetVisibility (Variables|Default|GetStaticMesh) false false)
    (Audio|PlaySoundatLocation "/Game/StarterContent/Audio/Explosion01.Explosion01" (Transformation|GetActorLocation) "0, 0, 0" 1.0 1.0 0.0 0 0 0 0)
    (Utilities|FlowControl|Delay 0.6)
    (Actor|DestroyActor)))

(event EventBeginPlay
  (if (Variables|Default|GetIsAutoMove)
    (Physics|SetSimulatePhysics (Variables|Default|GetStaticMesh) false)
    (Utilities|FlowControl|Delay 0.2)
    (Variables|Default|SetStartLocation (Variables|/Script/Engine.SceneComponent|GetRelativeLocation (Variables|Default|GetStaticMesh)))
    (bind _movevalue (Timeline|AutoMove Play)
      (:Update
        (Transformation|SetRelativeLocation (Variables|Default|GetStaticMesh) (Math|Vector|MakeVector (+ _movevalue (.x (Variables|Default|GetStartLocation))) (.y (Variables|Default|GetStartLocation)) (.z (Variables|Default|GetStartLocation))) false false)))))

(fn ConstructionScript)